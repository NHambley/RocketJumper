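; First-person player character for BlockBreaker, with movement, shooting, rocket jumping and wall jumping.
; BeginPlay attaches a spawned BP_Rifle, whose rates gate hitscan-style Shoot calls from the camera and RJ_Bullet spawns via delay-reset flags.
; Jumping in midair traces along three arrow components, mirrors the trace off the wall normal into a new velocity and turns the actor to it.
; Older hit-based wall-jump logic is disconnected or uncalled.
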(event `self.ReceiveTick`
  (params (DeltaSeconds :type "Float (single-precision)"))
  (bind _charactermovement (`self.CharacterMovement`))
  (if (`NavMovementComponent.IsFalling` _charactermovement)
    (set `CharacterMovementComponent.bOrientRotationToMovement` false _charactermovement)
    (else
      (set `CharacterMovementComponent.bOrientRotationToMovement` true _charactermovement))))

(event `InputAction|Jump`
  (params (Key :type "Key Structure"))
  (:`Pressed`
    (if (`NavMovementComponent.IsFalling` (`self.CharacterMovement`))
      (for _array_element (`self.ArrowArray`)
        (bind _returnvalue (`SceneComponent.K2_GetComponentLocation` _array_element))
        (bind _returnvalue_2 (+ _returnvalue (* (`SceneComponent.GetForwardVector` _array_element) 100.0)))
        (bind (_outhit _returnvalue_3) (`KismetSystemLibrary.LineTraceSingle` _returnvalue _returnvalue_2 "TraceTypeQuery1"))
        (if _returnvalue_3
          (bind _output_get (set `MovementComponent.Velocity` (+ (* (`KismetMathLibrary.Normal` (`KismetMathLibrary.MirrorVectorByNormal` (- _returnvalue_2 _returnvalue) (`.ImpactNormal` (`GameplayStatics.BreakHitResult` _outhit)))) 1000.0) (0.0 0.0 500.0)) (`self.CharacterMovement`)))
          (bind (_returnvalue_roll _returnvalue_pitch _returnvalue_yaw) (`KismetMathLibrary.BreakRotator` (`KismetMathLibrary.MakeRotFromXY` _output_get _output_get)))
          (`self.K2_SetActorRotation` (`KismetMathLibrary.MakeRotator` 0.0 0.0 _returnvalue_yaw))))
      (else
        (`self.LaunchCharacter` (0.0 0.0 500.0))))))

(event `self.ReceiveBeginPlay`
  (bind _returnvalue (`|SpawnActorFromClass` "/Game/BlockBreaker/Blueprints/GunThings/BP_Rifle.BP_Rifle_C" (`KismetMathLibrary.MakeTransform` (0.0 0.0 0.0)) "Undefined" "OverrideRootScale" null null))
  (bind _output_get (set `self.EquippedGun` _returnvalue))
  (`self.K2_AttachToComponent` _output_get (`self.GunLocation`) "None" "KeepRelative" "KeepRelative" "KeepRelative" true)
  (set `self.ArrowArray` (`|MakeArray` (`self.Arrow1`) (`self.Arrow2`) (`self.Arrow3`))))

(event `InputAxis|MoveRight`
  (params (AxisValue :type "Float (single-precision)"))
  (`self.AddMovementInput` (* (`self.GetActorRightVector`) (`self.MoveSpeed`)) AxisValue))

(event `InputAxis|MoveForward`
  (params (AxisValue :type "Float (single-precision)"))
  (`self.AddMovementInput` (* (`self.GetActorForwardVector`) (`self.MoveSpeed`)) AxisValue))

(event `InputAxis|LookVertical`
  (params (AxisValue :type "Float (single-precision)"))
  (`self.AddControllerPitchInput` AxisValue))

(event `InputAxis|LookHorizontal`
  (params (AxisValue :type "Float (single-precision)"))
  (`self.AddControllerYawInput` AxisValue))

(event `InputAxis|Shoot`
  (params (AxisValue :type "Float (single-precision)"))
  (bind _equippedgun (`self.EquippedGun`))
  (bind _fpscamera (`self.FpsCamera`))
  (bind _returnvalue (`SceneComponent.K2_GetComponentLocation` _fpscamera))
  (if (and (== AxisValue 1.0) (`self.CanShoot`))
    (`/Game/BlockBreaker/Blueprints/GunThings/BP_BaseGun.Shoot` _equippedgun _returnvalue (+ _returnvalue (* (`SceneComponent.GetForwardVector` _fpscamera) (`/Game/BlockBreaker/Blueprints/GunThings/BP_BaseGun.MaxBulletDistance` _equippedgun))))
    (set `self.CanShoot` false)
    (`KismetSystemLibrary.Delay` (`/Game/BlockBreaker/Blueprints/GunThings/BP_BaseGun.FireRate` (`self.EquippedGun`)))
    (set `self.CanShoot` true)))

(event `InputAxis|Rocket Jump`
  (params (AxisValue :type "Float (single-precision)"))
  (if (and (== AxisValue 1.0) (`self.CanRocket`))
    (`|SpawnActorFromClass` "/Game/BlockBreaker/Blueprints/RJ_Bullet.RJ_Bullet_C" (`SceneComponent.K2_GetComponentToWorld` (`/Game/BlockBreaker/Blueprints/GunThings/BP_BaseGun.RJ_Spawn` (`self.EquippedGun`))) "AlwaysSpawn" "OverrideRootScale" null null)
    (set `self.CanRocket` false)
    (`KismetSystemLibrary.Delay` (`/Game/BlockBreaker/Blueprints/GunThings/BP_BaseGun.RocketRate` (`self.EquippedGun`)))
    (set `self.CanRocket` true)))

(event `self.ReceiveHit`
  (params (MyComp :type "PrimitiveComponent Object Reference") (Other :type "Actor Object Reference") (OtherComp :type "PrimitiveComponent Object Reference") (bSelfMoved :type Boolean) (HitLocation :type "Vector Structure") (HitNormal :type "Vector Structure") (NormalImpulse :type "Vector Structure") (Hit :type "HitResult Structure (by ref)"))
  ;[1 1 1] Check collision with floor/wall, ignore gun collision so as to not get things weird, then check if they're wall jumping
)

(fn `GetJumpVector`
  (params (HitLocation :type "Vector Structure"))
  (set `self.JumpVector` (* (* (`KismetMathLibrary.Normal` (- (`self.K2_GetActorLocation`) HitLocation)) -1) (`self.Jump Velocity`))))

(fn `Player_Jump`
  (params (HitDirection :type "Vector Structure"))
  ;[1 1 1] if the player is jumping off a wall calculate a jump vector off the wall else just jump up.
  (if (not (`self.WallJump`))
    (bind _output_get (set `self.JumpVector` (0.0 0.0 1000.0)))
    (`self.LaunchCharacter` _output_get)))

(fn `UserConstructionScript`)